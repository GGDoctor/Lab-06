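; BOO is a Boo-style ghost enemy Actor that creeps toward the player while it is off screen.
; When WasRecentlyRendered is false, Tick moves it with VInterpTo toward the player pawn and reverses a timeline driving the material's Translucency parameter.
; An Interface event creates a dynamic material and starts the Speed timeline, whose value minus Interspeed sets the chase interpolation speed.
; Debug text prints the speed and approach.
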(event `self.ReceiveBeginPlay`)

(event `/Game/Blueprints/NewInterface.Interface`
  (bind _returnvalue (`PrimitiveComponent.CreateDynamicMaterialInstance` (`self.sphere`) 0 "/Game/StarterContent/Blueprints/Assets/MarioBoo_Mat.MarioBoo_Mat" "None"))
  (set `self.Translucent` _returnvalue)
  (bind (_direction _boo_time) (`Timeline|Speed` :!via `PlayFromStart`)
    (:`Update`
      (bind _output_get (set `self.subspeed` _boo_time))
      (`KismetSystemLibrary.PrintText` (`KismetTextLibrary.Conv_DoubleToText` (- _output_get (`self.interspeed`)) "HalfToEven") true false (struct :`G` 0.264687 :`B` 0.401042 :`A` 1.0) 0.01))))

(event `self.ReceiveTick`
  (params (DeltaSeconds :type "Float (single-precision)"))
  (if (not (`self.WasRecentlyRendered` 0.1))
    (`|ExecutionSequence`
      (:`then_0`
        (`KismetSystemLibrary.PrintString` "Boo is Coming" true true (struct :`G` 0.66 :`B` 1.0 :`A` 1.0) 0.5 "1")
        (`self.K2_SetActorLocationAndRotation` (`KismetMathLibrary.VInterpTo` (`self.K2_GetActorLocation`) (`self.K2_GetActorLocation` (`GameplayStatics.GetPlayerPawn` 0)) DeltaSeconds (- (stale `/Game/Blueprints/NewInterface.Interface` _output_get) (`self.interspeed`)))))
      (:`then_1`
        (bind (_direction _newtrack_0) (`Timeline|Boo_Mesh` :!via `Reverse`)
          (:`Update`
            (bind _output_get (set `self.blend value` _newtrack_0))
            (`MeshComponent.SetScalarParameterValueOnMaterials` (`self.sphere`) "Translucency" _output_get)))))))

(fn `UserConstructionScript`)