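; Door Blueprint that slides its DoorFrame between two positions when its Interface event fires.
; The event checks the Closed flag to play the Door timeline forward or in reverse.
; Each timeline update sets the frame's relative location by lerping from DoorStart to DoorEnd, then flips Closed, so the flag toggles on every update rather than once per interaction.
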(event `/Game/Blueprints/NewInterface.Interface`
  (if (`self.Closed?`)
    (bind (_direction _driver2) (`Timeline|Door` :!label _label)
      (:`Update`
        (`SceneComponent.K2_SetRelativeLocation` (`self.Door Frame`) (`KismetMathLibrary.VLerp` (`self.DoorStart`) (`self.DoorEnd`) _driver2) false false)
        (set `self.Closed?` (not (`self.Closed?`)))))
    (else
      (goto _label :!via `Reverse`))))

(fn `UserConstructionScript`)